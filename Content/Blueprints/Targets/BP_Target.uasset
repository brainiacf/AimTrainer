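; Shooting-gallery style target actor that moves or changes size, and awards match score when damaged.
; Construction randomizes its scale and picks a behaviour: horizontal move, vertical move or scale pulse.
; BeginPlay randomizes travel offset and timeline play rate, then one timeline lerps the mesh's relative location or scale.
; Damage passes points to its spawner, plays explosion sound and particles, then destroys the target.
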(event `self.ReceiveBeginPlay`
  (bind _returnvalue (`KismetMathLibrary.RandomFloatInRange` 100.0 250.0))
  (bind _actorscale (`self.ActorScale`))
  (switch `/Game/Blueprints/Targets/E_TargetBehaviour` (`self.TargetBehaviour`)
    (:`NewEnumerator1`
      (set `self.DestinationLocation` (`KismetMathLibrary.MakeVector` _returnvalue)))
    (:`NewEnumerator2`
      (set `self.DestinationLocation` (`KismetMathLibrary.MakeVector` 0.0 0.0 _returnvalue)))
    (:`NewEnumerator3`
      _))
  (`TimelineComponent.SetPlayRate` (`self.T_Move`) (/ 1.0 (`KismetMathLibrary.RandomFloatInRange` 1.5 3.0)))
  (bind (_direction _alpha) (`Timeline|T_Move` :!via `PlayFromStart`)
    (:`Update`
      (switch `/Game/Blueprints/Targets/E_TargetBehaviour` (`self.TargetBehaviour`)
        (:`NewEnumerator1`
          (`SceneComponent.K2_SetRelativeLocation` (`self.SM_Target`) (`KismetMathLibrary.VLerp` (0.0 0.0 0.0) (`self.DestinationLocation`) _alpha) false false :!label _label))
        (:`NewEnumerator2`
          (goto _label))
        (:`NewEnumerator3`
          (`SceneComponent.SetWorldScale3D` (`self.SM_Target`) (`KismetMathLibrary.VLerp` (`KismetMathLibrary.MakeVector` _actorscale _actorscale _actorscale) (`KismetMathLibrary.Conv_DoubleToVector` (* _actorscale 1.5)) _alpha)))))))

(event `/Game/Blueprints/Weapons/BPI_Damage.Receive Damage`
  (params (Points :type Integer))
  (bind _returnvalue (`SceneComponent.K2_GetComponentLocation` (`self.SM_Target`)))
  (`/Game/Blueprints/Targets/BP_Target_Spawner.UpdateMatchScore` (`self.SpawnerReference`) Points)
  (`GameplayStatics.PlaySoundAtLocation` "/Game/StarterContent/Audio/Explosion_Cue.Explosion_Cue" _returnvalue (struct) 1.0 1.0 0.0 null null null null)
  (`GameplayStatics.SpawnEmitterAtLocation` "/Game/StarterContent/Particles/P_Explosion.P_Explosion" _returnvalue (struct) (0.2 0.2 0.2))
  (`self.K2_DestroyActor`))

(fn `UserConstructionScript`
  ;[1 1 1] Setting Random Scale value for SM_Target
  (bind _output_get (set `self.ActorScale` (`KismetMathLibrary.RandomFloatInRange` 0.25 1.0)))
  (`SceneComponent.SetWorldScale3D` (`self.SM_Target`) (`KismetMathLibrary.MakeVector` _output_get _output_get _output_get))
  (set `self.TargetBehaviour` (cast `/Game/Blueprints/Targets/E_TargetBehaviour` (`KismetMathLibrary.Conv_IntToByte` (`KismetMathLibrary.RandomIntegerInRange` 1 3)))))