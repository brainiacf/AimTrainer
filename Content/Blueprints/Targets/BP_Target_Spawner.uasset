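; Target spawner for an aim trainer that runs a one-time timed round and tracks score.
; StartSpawning spawns an initial batch, then a looping timer adds camera-facing BP_Targets at random points in the SpawnArea box, capped by live count.
; Targets receive a spawner reference; UpdateMatchScore totals points into WB_Score.
; At round end it destroys targets and updates the session high in GI_AimTrainer and all-time high in a BPS_AimTrainerSave slot.
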(event `UpdateMatchScore`
  (params (Points :type Integer))
  (bind _output_get (set `self.MatchScore` (+ Points (`self.MatchScore`))))
  (`TextBlock.SetText` (`/Game/Blueprints/Targets/WB_Score.CurrentScore` (`self.WBScore`)) (`KismetTextLibrary.Conv_IntToText` _output_get)))

(event `self.ReceiveBeginPlay`
  (bind _returnvalue (`|CreateWidget` "/Game/Blueprints/Targets/WB_Score.WB_Score_C"))
  (bind _output_get (set `self.WBScore` _returnvalue))
  (`|ExecutionSequence`
    (:`then_0`
      (`UserWidget.AddToViewport` _output_get 0)
      (bind _asgi_aim_trainer (cast `/Game/Blueprints/FirstPersonTemplate/GI_AimTrainer` (`GameplayStatics.GetGameInstance`)))
      (`TextBlock.SetText` (`/Game/Blueprints/Targets/WB_Score.SessionHigh` (`self.WBScore`)) (`KismetTextLibrary.Conv_IntToText` (`/Game/Blueprints/FirstPersonTemplate/GI_AimTrainer.Score` _asgi_aim_trainer))))
    (:`then_1`
      (bind _returnvalue_2 (`GameplayStatics.DoesSaveGameExist` "Score"))
      (if _returnvalue_2
        (bind _returnvalue_3 (`GameplayStatics.LoadGameFromSlot` "Score"))
        (bind _asbps_aim_trainer_save (cast `/Game/Blueprints/FirstPersonTemplate/BPS_AimTrainerSave` _returnvalue_3))
        (`TextBlock.SetText` (`/Game/Blueprints/Targets/WB_Score.AllTimeHigh` (`self.WBScore`)) (`KismetTextLibrary.Conv_IntToText` (`/Game/Blueprints/FirstPersonTemplate/BPS_AimTrainerSave.HighScore` _asbps_aim_trainer_save)))
        (else
          (bind _returnvalue_4 (`GameplayStatics.CreateSaveGameObject` "/Game/Blueprints/FirstPersonTemplate/BPS_AimTrainerSave.BPS_AimTrainerSave_C"))
          (`GameplayStatics.SaveGameToSlot` _returnvalue_4 "Score"))))))

(event `StartSpawning`
  (bind _matchscore (`self.MatchScore`))
  (bind _matchscore_2 (`self.MatchScore`))
  (`/Engine/EditorBlueprintResources/StandardMacros.DoOnce` false
    (:`Completed`
      (bind _returnvalue (`KismetSystemLibrary.K2_SetTimerDelegate` (delegate `SpawnTarget`) 1.0 true))
      (set `self.TargetSpawner ` _returnvalue)
      (for _ (range 9)
        (`self.SpawnTarget`))
      (`KismetSystemLibrary.Delay` 10.0)
      (`KismetSystemLibrary.K2_ClearAndInvalidateTimerHandle` (`self.TargetSpawner `))
      (bind _outactors (`GameplayStatics.GetAllActorsOfClass` "/Game/Blueprints/Targets/BP_Target.BP_Target_C"))
      (for _array_element _outactors
        (`self.K2_DestroyActor` _array_element))
      (`|ExecutionSequence`
        (:`then_0`
          (bind _asgi_aim_trainer (cast `/Game/Blueprints/FirstPersonTemplate/GI_AimTrainer` (`GameplayStatics.GetGameInstance`)))
          (if (> _matchscore_2 (`/Game/Blueprints/FirstPersonTemplate/GI_AimTrainer.Score` _asgi_aim_trainer))
            (bind _output_get (set `/Game/Blueprints/FirstPersonTemplate/GI_AimTrainer.Score` _matchscore_2 _asgi_aim_trainer))
            (`TextBlock.SetText` (`/Game/Blueprints/Targets/WB_Score.SessionHigh` (`self.WBScore`)) (`KismetTextLibrary.Conv_IntToText` _output_get))))
        (:`then_1`
          (bind _returnvalue_2 (`GameplayStatics.LoadGameFromSlot` "Score"))
          (bind _asbps_aim_trainer_save (cast `/Game/Blueprints/FirstPersonTemplate/BPS_AimTrainerSave` _returnvalue_2))
          (if (< (`/Game/Blueprints/FirstPersonTemplate/BPS_AimTrainerSave.HighScore` _asbps_aim_trainer_save) _matchscore)
            (`TextBlock.SetText` (`/Game/Blueprints/Targets/WB_Score.AllTimeHigh` (`self.WBScore`)) (`KismetTextLibrary.Conv_IntToText` _matchscore))
            (set `/Game/Blueprints/FirstPersonTemplate/BPS_AimTrainerSave.HighScore` _matchscore _asbps_aim_trainer_save)
            (`GameplayStatics.SaveGameToSlot` _asbps_aim_trainer_save "Score")))))))

(event `SpawnTarget`
  (bind _spawnarea (`self.SpawnArea`))
  (bind _outactors (`GameplayStatics.GetAllActorsOfClass` "/Game/Blueprints/Targets/BP_Target.BP_Target_C"))
  (if (<= (`KismetArrayLibrary.Array_Length` _outactors) 10)
    (bind _output_get (set `self.SpawnLocation` (`KismetMathLibrary.RandomPointInBoundingBox` (`SceneComponent.K2_GetComponentLocation` _spawnarea) (`BoxComponent.GetScaledBoxExtent` _spawnarea))))
    (bind (_returnvalue_roll _returnvalue_pitch _returnvalue_yaw) (`KismetMathLibrary.BreakRotator` (`KismetMathLibrary.FindLookAtRotation` _output_get (`SceneComponent.K2_GetComponentLocation` (`PlayerCameraManager.TransformComponent` (`GameplayStatics.GetPlayerCameraManager` 0))))))
    (`|SpawnActorFromClass` "/Game/Blueprints/Targets/BP_Target.BP_Target_C" (`KismetMathLibrary.MakeTransform` _output_get (`KismetMathLibrary.MakeRotator` _returnvalue_roll _returnvalue_pitch (- _returnvalue_yaw 90.0))) "Undefined" "MultiplyWithRoot" null self null)))

(fn `UserConstructionScript`
  (`BoxComponent.SetBoxExtent` (`self.SpawnArea`) (`self.In Box Extent`) true))